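; BP_Guardian1 is an AI guardian character that responds to camera alerts and can be temporarily frozen by damage.
; On BeginPlay it caches the player, its Guardian_Controller and Blackboard, then binds to the referenced camera's alert dispatcher.
; The Alert event writes the ping location to the Blackboard's TargetLocation key.
; Any damage disables movement for a timed freeze before restoring walking, and completes Quest2 on the player.
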(event Custom|Unfreeze
  (Variables|Default|SetFreeze false)
  (Pawn|Components|CharacterMovement|SetMovementMode (Variables|Character|GetCharacterMovement) "MOVE_Walking" 0))

(event Custom|Alert
  (params (PingLocation :type Vector))
  ;[0.15 0.15 0.15 0.5] Alerte à distance
  (AI|Components|Blackboard|SetValueasVector (Variables|Default|GetBlackboard) (Utilities|Name|MakeLiteralName "TargetLocation") PingLocation)
  (Development|PrintText "Hello"))

(event EventBeginPlay
  ;[0.15 0.15 0.15 0.5] Initialization
  (bind _returnvalue (Actor|GetActorOfClass "/Game/02-Blueprints/Player/BP_Player.BP_Player_C"))
  (Variables|Default|SetBP%20Player _returnvalue)
  (bind _asguardian_controller (Utilities|Casting|CastToGuardian_Controller (Pawn|GetController)))
  (Variables|Default|SetAs%20Guardian%20Controller _asguardian_controller)
  (Variables|Default|SetBlackboard (AI|GetBlackboard 0))
  (bind _cameraref (Variables|Default|GetCameraRef)
    (:then
      (EventDispatchers|BindEventtoAlertDispatch _cameraref (EventDispatchers|CreateEvent :!event Custom|Alert)))
    (:else)))

(event Game|Damage|EventAnyDamage
  (params (Damage :type Float%20%28single-precision%29) (DamageType :type Damage%20Type%20Object%20Reference) (InstigatedBy :type Controller%20Object%20Reference) (DamageCauser :type Actor%20Object%20Reference))
  (Variables|Default|SetFreeze true)
  (Pawn|Components|CharacterMovement|DisableMovement (Variables|Character|GetCharacterMovement))
  (Utilities|FlowControl|Sequence
    (:then_0
      (Utilities|FlowControl|Delay 2e+01)
      (CallFunction|Unfreeze))
    (:then_1
      (Default|CompletedQuest (Variables|Default|GetBP%20Player) "Quest2"))))

(fn ConstructionScript)