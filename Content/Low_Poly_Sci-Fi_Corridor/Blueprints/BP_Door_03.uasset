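; Sliding double door for the labyrinth that opens when the player or a BP_Guardian1 capsule enters its trigger box, unless it is locked.
; A timeline slides the left and right panels between closed and open positions with sound, then reverses on overlap end regardless of lock state.
; On BeginPlay it binds to BP_Labyrinth's UnlockAll event to clear its lock.
; The construction script applies a configurable material to all three meshes.
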(event OnComponentEndOverlap(Box)
  (params (OverlappedComponent :type Primitive%20Component%20Object%20Reference) (OtherActor :type Actor%20Object%20Reference) (OtherComp :type Primitive%20Component%20Object%20Reference) (OtherBodyIndex :type Integer))
  (Utilities|FlowControl|Sequence
    (:then_0
      (bind _asbp_player (Utilities|Casting|CastToBP_Player OtherActor))
      (if (== (Variables|/Script/Engine.Character|GetCapsuleComponent _asbp_player) OtherComp)
        (Audio|Components|Audio|Play (Variables|Default|GetClose) 0.0 :!label _label)
        (bind _newtrack_0 (Timeline|Door_Slide Reverse)
          (:Update
            (Transformation|SetRelativeLocation (Variables|Default|GetSM_Door_03_B_Left) (Math|Vector|Lerp(Vector) (Variables|Default|GetDoor_Closed_Left) (Variables|Default|GetDoor_Open_Left) _newtrack_0) false false)
            (Transformation|SetRelativeLocation (Variables|Default|GetSM_Door_03_C_Right) (Math|Vector|Lerp(Vector) (Variables|Default|GetDoor_Closed_Right) (Variables|Default|GetDoor_Open_Right) _newtrack_0) false false)))))
    (:then_1
      (bind _asbp_guardian_1 (Utilities|Casting|CastToBP_Guardian1 OtherActor))
      (if (== (Variables|/Script/Engine.Character|GetCapsuleComponent _asbp_guardian_1) OtherComp)
        (goto _label)))))

(event OnComponentBeginOverlap(Box)
  (params (OverlappedComponent :type Primitive%20Component%20Object%20Reference) (OtherActor :type Actor%20Object%20Reference) (OtherComp :type Primitive%20Component%20Object%20Reference) (OtherBodyIndex :type Integer) (bFromSweep :type Boolean) (SweepResult :type Hit%20Result%20Structure%20%28by%20ref%29))
  (Utilities|FlowControl|Sequence
    (:then_0
      (bind _asbp_player (Utilities|Casting|CastToBP_Player OtherActor))
      (if (== (Variables|/Script/Engine.Character|GetCapsuleComponent _asbp_player) OtherComp)
        (if (not (Variables|Default|Getis%20Lock)) :!label _label
          (Audio|Components|Audio|Play (Variables|Default|GetOpen) 0.2)
          (bind _newtrack_0 (Timeline|Door_Slide Play)
            (:Update
              (Transformation|SetRelativeLocation (Variables|Default|GetSM_Door_03_B_Left) (Math|Vector|Lerp(Vector) (Variables|Default|GetDoor_Closed_Left) (Variables|Default|GetDoor_Open_Left) _newtrack_0) false false)
              (Transformation|SetRelativeLocation (Variables|Default|GetSM_Door_03_C_Right) (Math|Vector|Lerp(Vector) (Variables|Default|GetDoor_Closed_Right) (Variables|Default|GetDoor_Open_Right) _newtrack_0) false false))))))
    (:then_1
      (bind _asbp_guardian_1 (Utilities|Casting|CastToBP_Guardian1 OtherActor))
      (if (== (Variables|/Script/Engine.Character|GetCapsuleComponent _asbp_guardian_1) OtherComp)
        (goto _label)))))

(event Custom|Unlock
  (Variables|Default|Setis%20Lock false))

(event EventBeginPlay
  (bind _returnvalue (Actor|GetActorOfClass "/Game/02-Blueprints/Labyrinth/BP_Labyrinth.BP_Labyrinth_C"))
  (EventDispatchers|BindEventtoUnlockAll _returnvalue (delegate Custom|Unlock)))

(fn ConstructionScript
  (Rendering|Material|SetMaterial (Variables|Default|GetSM_Door_03_A) 0 (Variables|Default|GetMaterial)))