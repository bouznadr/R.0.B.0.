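; BP_Fan_03_A is a spinning fan prop from the low-poly sci-fi corridor set, with sound.
; The construction script applies the Material variable to both fan meshes at slot 0.
; BeginPlay starts the Audio component, and Tick rolls the Arrow component locally by Speed scaled by delta time, giving frame-rate-independent rotation.
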(event EventBeginPlay
  (Audio|Components|Audio|Play (Variables|Default|GetAudio) 0.0))

(event Collision|EventActorBeginOverlap
  (params (OtherActor :type Actor%20Object%20Reference)))

(event EventTick
  (params (DeltaSeconds :type Float%20%28single-precision%29))
  (Transformation|AddLocalRotation (Variables|Default|GetArrow) (* (Math|Rotator|MakeRotator (Variables|Default|GetSpeed) 0.0 0.0) DeltaSeconds) false false))

(fn ConstructionScript
  (Rendering|Material|SetMaterial (Variables|Default|GetSM_Fan_02_A) 0 (Variables|Default|GetMaterial)))