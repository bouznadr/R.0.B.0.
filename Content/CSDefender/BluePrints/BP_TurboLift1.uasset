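; BP_TurboLift1 is a lift whose platform the player toggles between two positions by overlapping its Cylinder trigger.
; A FlipFlop alternates the direction on each BP_Player overlap, stopping the opposite MoveComponentTo, then moving the platform to the end or start relative transform after a short delay.
; A steam sound fades in before each move and fades out when the move completes.
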(event OnComponentBeginOverlap(Cylinder)
  (params (OverlappedComponent :type Primitive%20Component%20Object%20Reference) (OtherActor :type Actor%20Object%20Reference) (OtherComp :type Primitive%20Component%20Object%20Reference) (OtherBodyIndex :type Integer) (bFromSweep :type Boolean) (SweepResult :type Hit%20Result%20Structure%20%28by%20ref%29))
  (bind _over_time_0 (Variables|Default|GetOver%20Time_0))
  (bind _startrelative_location (Variables|Default|GetStartRelative%20Location))
  (bind _endtrelative_location_0 (Variables|Default|GetEndtRelative%20Location_0))
  (bind _sm_turboliftplatform (Variables|Default|GetSM_TurboLiftPlatform))
  (Utilities|Casting|CastToBP_Player OtherActor)
  (Utilities|FlowControl|FlipFlop
    (:A
      (Utilities|FlowControl|Sequence
        (:then_0
          (goto _label_2 Stop))
        (:then_1
          (Audio|Components|Audio|FadeIn (Variables|Default|GetSteam01_Cue) 0.1 1.0 0.0 "Linear" :!class /Script/Engine.AudioComponent)
          (Utilities|FlowControl|Delay 1.0)
          (Components|MoveComponentTo _sm_turboliftplatform (.location _endtrelative_location_0) (.rotation _endtrelative_location_0) false false _over_time_0 false :!label _label))))
    (:B
      (Utilities|FlowControl|Sequence
        (:then_0
          (goto _label Stop))
        (:then_1
          (Audio|Components|Audio|FadeIn (Variables|Default|GetSteam01_Cue) 0.1 1.0 0.0 "Linear" :!class /Script/Engine.AudioComponent)
          (Utilities|FlowControl|Delay 1.0)
          (Components|MoveComponentTo _sm_turboliftplatform (.location _startrelative_location) (.rotation _startrelative_location) false false _over_time_0 false :!label _label_2)))))
  (Audio|Components|Audio|FadeOut (Variables|Default|GetSteam01_Cue) 0.1 0.0 "Linear" :!class /Script/Engine.AudioComponent))

(fn ConstructionScript)