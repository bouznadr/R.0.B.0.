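; Automatic two-leaf corridor door that opens when BP_ThirdPersonCharacter enters DoorTrigger and closes when it leaves.
; Each overlap event starts MoveComponentTo on both leaves toward end or start markers, with ease-out on opening, and stops the opposing moves so direction can reverse mid-motion.
; Light01Cue fades in as movement starts and fades out when the right leaf's move completes.
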(event OnComponentBeginOverlap(DoorTrigger)
  (params (OverlappedComponent :type Primitive%20Component%20Object%20Reference) (OtherActor :type Actor%20Object%20Reference) (OtherComp :type Primitive%20Component%20Object%20Reference) (OtherBodyIndex :type Integer) (bFromSweep :type Boolean) (SweepResult :type Hit%20Result%20Structure%20%28by%20ref%29))
  (bind _sm_coridordoorleft (Variables|Default|GetSM_CoridorDoorLeft))
  (bind _leftdoorstartpos (Variables|Default|GetLeftDoorStartPos))
  (bind _leftdoorendpos (Variables|Default|GetLeftDoorEndPos))
  (bind _sm_coridordoorright (Variables|Default|GetSM_CoridorDoorRight))
  (bind _rightdoorendpos (Variables|Default|GetRightDoorEndPos))
  (bind _rightdoorstartpos (Variables|Default|GetRightDoorStartPos))
  (Utilities|Casting|CastToBP_ThirdPersonCharacter OtherActor)
  (Audio|Components|Audio|FadeIn (Variables|Default|GetLight01_Cue) 0.1 1.0 0.0 "Linear" :!class /Script/Engine.AudioComponent)
  (Utilities|FlowControl|Sequence
    (:then_0
      (Components|MoveComponentTo _sm_coridordoorleft (.location _leftdoorendpos) (.rotation _leftdoorendpos) true false 1.0 false)
      (Components|MoveComponentTo _sm_coridordoorright (.location _rightdoorendpos) (.rotation _rightdoorendpos) true false 1.0 false :!label _label)
      (Audio|Components|Audio|FadeOut (Variables|Default|GetLight01_Cue) 0.1 0.0 "Linear" :!class /Script/Engine.AudioComponent))
    (:then_1
      (goto _label))
    (:then_2
      (Components|MoveComponentTo _sm_coridordoorleft (.location _leftdoorstartpos) (.rotation _leftdoorstartpos) false false 1.0 false) ; enters at Stop
    )
    (:then_3
      (Components|MoveComponentTo _sm_coridordoorright (.location _rightdoorstartpos) (.rotation _rightdoorstartpos) false false 1.0 false) ; enters at Stop
    )))

(event OnComponentEndOverlap(DoorTrigger)
  (params (OverlappedComponent :type Primitive%20Component%20Object%20Reference) (OtherActor :type Actor%20Object%20Reference) (OtherComp :type Primitive%20Component%20Object%20Reference) (OtherBodyIndex :type Integer))
  (bind _sm_coridordoorleft (Variables|Default|GetSM_CoridorDoorLeft))
  (bind _leftdoorstartpos (Variables|Default|GetLeftDoorStartPos))
  (bind _leftdoorendpos (Variables|Default|GetLeftDoorEndPos))
  (bind _sm_coridordoorright (Variables|Default|GetSM_CoridorDoorRight))
  (bind _rightdoorendpos (Variables|Default|GetRightDoorEndPos))
  (bind _rightdoorstartpos (Variables|Default|GetRightDoorStartPos))
  (Utilities|Casting|CastToBP_ThirdPersonCharacter OtherActor)
  (Audio|Components|Audio|FadeIn (Variables|Default|GetLight01_Cue) 0.1 1.0 0.0 "Linear" :!class /Script/Engine.AudioComponent)
  (Utilities|FlowControl|Sequence
    (:then_0
      (Components|MoveComponentTo _sm_coridordoorleft (.location _leftdoorstartpos) (.rotation _leftdoorstartpos) false false 1.0 false)
      (Components|MoveComponentTo _sm_coridordoorright (.location _rightdoorstartpos) (.rotation _rightdoorstartpos) false false 1.0 false :!label _label)
      (Audio|Components|Audio|FadeOut (Variables|Default|GetLight01_Cue) 0.1 0.0 "Linear" :!class /Script/Engine.AudioComponent))
    (:then_1
      (goto _label))
    (:then_2
      (Components|MoveComponentTo _sm_coridordoorleft (.location _leftdoorendpos) (.rotation _leftdoorendpos) true false 1.0 false) ; enters at Stop
    )
    (:then_3
      (Components|MoveComponentTo _sm_coridordoorright (.location _rightdoorendpos) (.rotation _rightdoorendpos) true false 1.0 false) ; enters at Stop
    )))

(fn ConstructionScript)