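; BP_AlarmLight is an alarm light that turns on when the player is detected.
; On BeginPlay it finds BP_Player and binds to its detection-changed event.
; When detected, LightOn unhides the PointLight and delays for the AlarmDuration read from BP_Camera.
; After the delay it sets the light visible again rather than hiding it, so nothing here switches it off.
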(event Custom|LightOn
  (params (Player%20is%20Detected? :type Boolean))
  (if Player%20is%20Detected?
    (Development|SetHiddeninGame (Variables|Default|GetPointLight) false false)
    (bind _returnvalue (Actor|GetActorOfClass "/Game/02-Blueprints/BP_Camera.BP_Camera_C"))
    (Utilities|FlowControl|Delay (Variables|/Game/02-Blueprints/BP_Camera.BP_Camera_C|GetAlarm%20Duration _returnvalue))
    (Development|SetHiddeninGame (Variables|Default|GetPointLight) false false)))

(event EventBeginPlay
  (bind _returnvalue (Actor|GetActorOfClass "/Game/02-Blueprints/Player/BP_Player.BP_Player_C"))
  (EventDispatchers|BindEventtoOnDetectionChanged _returnvalue (EventDispatchers|CreateEvent :!event Custom|LightOn)))

(fn ConstructionScript)