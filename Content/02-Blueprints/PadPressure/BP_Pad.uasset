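; BP_Pad is a weight-sensitive pressure pad that sinks as overlapping objects load it and sends its load fraction to connected actors.
; Box overlaps update a weight clamped to a target using component mass, though map entries are removed right after adding, so end overlaps zero the weight.
; Percentage changes notify connected actors and enable Tick, which eases the pad's height and disables itself once settled.
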(event OnComponentBeginOverlap(Box)
  (params (OverlappedComponent :type Primitive%20Component%20Object%20Reference) (OtherActor :type Actor%20Object%20Reference) (OtherComp :type Primitive%20Component%20Object%20Reference) (OtherBodyIndex :type Integer) (bFromSweep :type Boolean) (SweepResult :type Hit%20Result%20Structure%20%28by%20ref%29))
  (CallFunction|ObjectinPad OtherActor OtherComp true)
  (CallFunction|UpdateStats))

(event OnComponentEndOverlap(Box)
  (params (OverlappedComponent :type Primitive%20Component%20Object%20Reference) (OtherActor :type Actor%20Object%20Reference) (OtherComp :type Primitive%20Component%20Object%20Reference) (OtherBodyIndex :type Integer))
  (CallFunction|ObjectinPad OtherActor OtherComp false)
  (CallFunction|UpdateStats))

(event EventBeginPlay)

(event Collision|EventActorBeginOverlap
  (params (OtherActor :type Actor%20Object%20Reference)))

(event EventTick
  (params (DeltaSeconds :type Float%20%28single-precision%29))
  (if (== (Variables|Default|GetCurrent%20weight%20percent) (Variables|Default|GetPad%20offset))
    (Actor|Tick|SetActorTickEnabled false)
    (else
      (Variables|Default|SetPad%20offset (Math|Interpolation|FInterpTo (Variables|Default|GetPad%20offset) (Variables|Default|GetCurrent%20weight%20percent) (Utilities|Time|GetWorldDeltaSeconds) 1e+01))
      (Variables|Default|SetPad%20Position (Math|Vector|MakeVector 0.0 0.0 (Math|Float|Lerp 1e+02 2e+01 (Variables|Default|GetPad%20offset))))
      (Transformation|SetRelativeLocation (Variables|Default|GetPad) (Variables|Default|GetPad%20Position) false false))))

(fn ConstructionScript)

(fn ObjectinPad
  (params (In%20actor :type Actor%20Object%20Reference) (in%20comp :type Primitive%20Component%20Object%20Reference) (Plus :type Boolean))
  (bind _object_on_pad__weight (Variables|Default|GetObject%20on%20pad/%20weight))
  (bind _value (Utilities|Map|Find _object_on_pad__weight In%20actor))
  (if Plus
    (Utilities|Map|Add (Variables|Default|GetObject%20on%20pad/%20weight) In%20actor (Physics|GetMass in%20comp)))
  (if (Utilities|Map|IsEmpty (Variables|Default|GetObject%20on%20pad/%20weight))
    (Variables|Default|SetCurrent%20Weight 0.0)
    (else
      (Variables|Default|SetCurrent%20Weight (Math|Float|Clamp(Float) (+ (Variables|Default|GetCurrent%20Weight) (select Plus _value (* _value -1.0))) 0.0 (Variables|Default|GetTarget%20Weight)))))
  (if Plus
    (Utilities|Map|Remove (Variables|Default|GetObject%20on%20pad/%20weight) In%20actor)))

(fn UpdateStats
  (bind _current_weight (Variables|Default|GetCurrent%20Weight))
  (bind _target_weight (Variables|Default|GetTarget%20Weight))
  (bind _returnvalue (/ _current_weight _target_weight))
  (bind _returnvalue_2 (Math|Float|Clamp(Float) _returnvalue))
  (if (not (== (Variables|Default|GetCurrent%20weight%20percent) _returnvalue_2))
    (Variables|Default|SetCurrent%20weight%20percent _returnvalue_2)
    (Actor|Tick|SetActorTickEnabled true)
    (for _array_element (Variables|Default|GetConnected%20Actor)
      (Class|BPIWeight|CurrentWeightValues(Message) (Utilities|ResolveSoftReference _array_element) (Variables|Default|GetCurrent%20weight%20percent)))))