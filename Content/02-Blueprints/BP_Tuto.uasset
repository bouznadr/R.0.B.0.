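; BP_Tuto is a one-shot tutorial actor that shows a tutorial entry on the player's HUD.
; It caches PlayerHUD from BP_Player one second after BeginPlay.
; When LoadTuto runs with IsPlayerlook set, it looks up RowName in the FS_Tuto data table and passes the title, description, video, image and media source to UpdateTuto.
; It then clears the flag and destroys itself.
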(event EventBeginPlay
  (Utilities|FlowControl|Delay 1.0)
  (bind _returnvalue (Actor|GetActorOfClass "/Game/02-Blueprints/Player/BP_Player.BP_Player_C"))
  (Variables|Default|SetPlayer%20HUD (Variables|/Game/02-Blueprints/Player/BP_Player.BP_Player_C|GetPlayer%20HUD _returnvalue)))

(fn ConstructionScript)

(fn LoadTuto
  (if (Variables|Default|GetIsPlayerlook)
    (bind _returnvalue (Utilities|GetDataTableRow "/Game/05-DataTable/FS_Tuto.FS_Tuto" (Variables|Default|GetRow%20Name))
      (:then
        (Default|UpdateTuto (Variables|Default|GetPlayer%20HUD) (.Titre (Utilities|Struct|BreakS_Tuto _returnvalue)) (.Video (Utilities|Struct|BreakS_Tuto _returnvalue)) (.Descriptions (Utilities|Struct|BreakS_Tuto _returnvalue)) (.image (Utilities|Struct|BreakS_Tuto _returnvalue)) (.mediasource (Utilities|Struct|BreakS_Tuto _returnvalue)))
        (Variables|Default|SetIsPlayerlook false)
        (Actor|DestroyActor)))))