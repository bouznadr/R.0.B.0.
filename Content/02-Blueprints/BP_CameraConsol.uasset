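; Camera console actor that shows a camera control widget to the player and tracks a four-stage progress sequence.
; The widget is created at BeginPlay, then added to or removed from the viewport as the player's capsule enters or leaves the trigger box.
; CheckCam starts one timeline run unless busy or finished, lerping the current stage's value from 100 to 0.
; Each completed run advances the index, and the fourth marks the console finished.
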(event OnComponentBeginOverlap(Box)
  (params (OverlappedComponent :type Primitive%20Component%20Object%20Reference) (OtherActor :type Actor%20Object%20Reference) (OtherComp :type Primitive%20Component%20Object%20Reference) (OtherBodyIndex :type Integer) (bFromSweep :type Boolean) (SweepResult :type Hit%20Result%20Structure%20%28by%20ref%29))
  (bind _asbp_player (Utilities|Casting|CastToBP_Player OtherActor))
  (if (== (Variables|/Script/Engine.Character|GetCapsuleComponent _asbp_player) OtherComp)
    (UserInterface|Viewport|AddtoViewport (Variables|Default|GetCamRef) 0)))

(event OnComponentEndOverlap(Box)
  (params (OverlappedComponent :type Primitive%20Component%20Object%20Reference) (OtherActor :type Actor%20Object%20Reference) (OtherComp :type Primitive%20Component%20Object%20Reference) (OtherBodyIndex :type Integer))
  (bind _asbp_player (Utilities|Casting|CastToBP_Player OtherActor))
  (if (== (Variables|/Script/Engine.Character|GetCapsuleComponent _asbp_player) OtherComp)
    (Widget|RemovefromParent (Variables|Default|GetCamRef))))

(event Custom|CheckCam
  (if (not (Variables|Default|GetIsfinished?))
    (if (not (Variables|Default|GetInprogress?))
      (CallFunction|Start))))

(event Custom|Start
  (Variables|Default|SetInprogress? true)
  (bind _nouvelle_piste_0 (Timeline|Chronologie PlayFromStart)
    (:Update
      (if (== (Variables|Default|GetProgressIndex) 0)
        (Variables|Default|SetProgressIndex_0 (Math|Float|Lerp 1e+02 0.0 _nouvelle_piste_0))
        (elif (== (Variables|Default|GetProgressIndex) 1)
          (Variables|Default|SetProgressIndex_1 (Math|Float|Lerp 1e+02 0.0 _nouvelle_piste_0))
          (elif (== (Variables|Default|GetProgressIndex) 2)
            (Variables|Default|SetProgressIndex_2 (Math|Float|Lerp 1e+02 0.0 _nouvelle_piste_0))
            (elif (== (Variables|Default|GetProgressIndex) 3)
              (Variables|Default|SetProgressIndex_3 (Math|Float|Lerp 1e+02 0.0 _nouvelle_piste_0)))))))
    (:Finished
      (Variables|Default|SetProgressIndex (+ (Variables|Default|GetProgressIndex) 1))
      (Variables|Default|SetInprogress? false)
      (if (>= (Variables|Default|GetProgressIndex) 4)
        (Variables|Default|SetIsfinished? true)))))

(event EventBeginPlay
  (bind _returnvalue (UserInterface|CreateWidget "/Game/02-Blueprints/UI/WBP_CameraControl.WBP_CameraControl_C"))
  (Variables|Default|SetCamRef _returnvalue)
  (Variables|Default|SetProgressIndex 0))

(fn ConstructionScript)