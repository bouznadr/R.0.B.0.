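; BP_PickUP_GravityGun is a pickup item that gives the player use of the gravity gun.
; When used, it calls ActivateGravityGun on the player's GravityGun, then CompleteQuest on the player's QuestManager with the argument "None".
; It relies on its parent class for the rest, with BeginPlay and the construction script only calling the parent versions.
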(event EventBeginPlay
  (|CallParentFunction))

(event Collision|EventActorBeginOverlap
  (params (OtherActor :type Actor%20Object%20Reference))
  (|CallParentFunction OtherActor) ; Ce nœud est désactivé et ne sera pas appelé.\nFaites glisser les broches pour générer des fonctionnalités.
)

(event EventTick
  (params (DeltaSeconds :type Float%20%28single-precision%29))
  (|CallParentFunction DeltaSeconds) ; Ce nœud est désactivé et ne sera pas appelé.\nFaites glisser les broches pour générer des fonctionnalités.
)

(event EventUsePickedItem
  (bind _bp_player (Variables|Default|GetBP%20Player))
  (Class|GravityGunComponent|ActivateGravityGun (Variables|/Game/02-Blueprints/BP_Player.BP_Player_C|GetGravityGun _bp_player))
  (Class|QuestManagerComponent|CompleteQuest (Variables|/Game/02-Blueprints/BP_Player.BP_Player_C|GetQuestManager _bp_player) "None"))

(fn ConstructionScript
  (|CallParentFunction))