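; BP_Door is a sliding two-panel corridor door with lock and super-lock flags that block opening.
; ActiveDoor_Event opens it through a DoOnce-gated timeline with sound, then closes it after delays.
; A box trigger separately opens it for BP_Guardian1's capsule and reverses that timeline on exit.
; Monitor materials reflect the lock at construction and on debug-key T toggles, while BP_Labyrinth's unlock-all event clears only the lock flag.
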(event OnComponentBeginOverlap(Box)
  (params (OverlappedComponent :type Primitive%20Component%20Object%20Reference) (OtherActor :type Actor%20Object%20Reference) (OtherComp :type Primitive%20Component%20Object%20Reference) (OtherBodyIndex :type Integer) (bFromSweep :type Boolean) (SweepResult :type Hit%20Result%20Structure%20%28by%20ref%29))
  (bind _asbp_guardian_1 (Utilities|Casting|CastToBP_Guardian1 OtherActor))
  (if (== (Variables|/Script/Engine.Character|GetCapsuleComponent _asbp_guardian_1) OtherComp)
    (if (not (Variables|Default|GetisSuperLock))
      (if (not (Variables|Default|GetIsLock))
        (if (not (Variables|Default|GetOpenDoor))
          (Audio|Components|Audio|Play (Variables|Default|GetAudio) 0.35)
          (bind _newtrack_2 (Timeline|Chronologie Play)
            (:Update
              (Transformation|SetRelativeLocation (Variables|Default|GetSM_CoridorDoorRight) (Math|Vector|MakeVector (Math|Float|Lerp 0.0 (Variables|Default|GetOpenDoorRight) _newtrack_2) 0.0 0.0) false false)
              (Transformation|SetRelativeLocation (Variables|Default|GetSM_CoridorDoorLeft) (Math|Vector|MakeVector (Math|Float|Lerp 0.0 (Variables|Default|GetOpeDoorLeft) _newtrack_2) 0.0 0.0) false false))))))))

(event OnComponentEndOverlap(Box)
  (params (OverlappedComponent :type Primitive%20Component%20Object%20Reference) (OtherActor :type Actor%20Object%20Reference) (OtherComp :type Primitive%20Component%20Object%20Reference) (OtherBodyIndex :type Integer))
  (bind _asbp_guardian_1 (Utilities|Casting|CastToBP_Guardian1 OtherActor))
  (if (== (Variables|/Script/Engine.Character|GetCapsuleComponent _asbp_guardian_1) OtherComp)
    (Audio|Components|Audio|Play (Variables|Default|GetAudio1) 0.35)
    (bind _newtrack_2 (Timeline|Chronologie Reverse)
      (:Update
        (Transformation|SetRelativeLocation (Variables|Default|GetSM_CoridorDoorRight) (Math|Vector|MakeVector (Math|Float|Lerp 0.0 (Variables|Default|GetOpenDoorRight) _newtrack_2) 0.0 0.0) false false)
        (Transformation|SetRelativeLocation (Variables|Default|GetSM_CoridorDoorLeft) (Math|Vector|MakeVector (Math|Float|Lerp 0.0 (Variables|Default|GetOpeDoorLeft) _newtrack_2) 0.0 0.0) false false)))))

(event Custom|ActiveDoor_Event
  ;[0.04424 0.02965 0.15 0.5] Open Door
  (if (not (Variables|Default|GetisSuperLock))
    (if (not (Variables|Default|GetIsLock))
      (Variables|Default|SetOpenDoor true)
      (Audio|Components|Audio|Play (Variables|Default|GetAudio) 0.35)
      (Utilities|FlowControl|DoOnce false :!label _label
        (:Completed
          (bind _newtrack_2 (Timeline|Open_Door PlayFromStart)
            (:Update
              (Transformation|SetRelativeLocation (Variables|Default|GetSM_CoridorDoorRight) (Math|Vector|MakeVector (Math|Float|Lerp 0.0 (Variables|Default|GetOpenDoorRight) _newtrack_2) 0.0 0.0) false false)
              (Transformation|SetRelativeLocation (Variables|Default|GetSM_CoridorDoorLeft) (Math|Vector|MakeVector (Math|Float|Lerp 0.0 (Variables|Default|GetOpeDoorLeft) _newtrack_2) 0.0 0.0) false false)
              (Utilities|FlowControl|Delay 1.0)
              ;[0.0204 0.15 0.03553 0.5] Clos Door
              (Utilities|FlowControl|Delay 5.0)
              (Audio|Components|Audio|Play (Variables|Default|GetAudio1) 0.0)
              (bind _newtrack_0 (Timeline|Timeline PlayFromStart)
                (:Update
                  (Transformation|SetRelativeLocation (Variables|Default|GetSM_CoridorDoorRight) (Math|Vector|MakeVector (Math|Float|Lerp 0.0 -19.0 _newtrack_0) 0.0 0.0) false false)
                  (Transformation|SetRelativeLocation (Variables|Default|GetSM_CoridorDoorLeft) (Math|Vector|MakeVector (Math|Float|Lerp 0.0 19.0 _newtrack_0) 0.0 0.0) false false)
                  (Utilities|FlowControl|Delay 1.0)
                  (Transformation|SetRelativeLocation (Variables|Default|GetSM_CoridorDoorRight) (Math|Vector|MakeVector (Variables|Default|GetClosDoorRight) 0.0 0.0) false false)
                  (Transformation|SetRelativeLocation (Variables|Default|GetSM_CoridorDoorLeft) (Math|Vector|MakeVector (Variables|Default|GetClosDoorLeft) 0.0 0.0) false false)
                  (Variables|Default|SetOpenDoor false)
                  (goto _label Reset))))))))))

(event Custom|Unlock
  (Variables|Default|SetIsLock false))

(event EventBeginPlay
  (bind _returnvalue (Actor|GetActorOfClass "/Game/02-Blueprints/Labyrinth/BP_Labyrinth.BP_Labyrinth_C"))
  (EventDispatchers|BindEventtoUnlockAll _returnvalue (delegate Custom|Unlock)))

(event Input|KeyboardEvents|DebugKeyT
  (params (Key :type Key%20Structure :default "None") (ActionValue :type Input%20Action%20Value%20Structure))
  (bind _monitor1 (Variables|Default|GetMonitor1))
  (:Pressed
    (bind _isa (Utilities|FlowControl|FlipFlop)
      (:A
        _)
      (:B
        _))
    (bind _output_get (Variables|Default|SetIsLock _isa))
    (if _output_get
      (Rendering|Material|SetMaterial _monitor1 1 "/Game/Low_Poly_Sci-Fi_Corridor/Materials/Alternate/Green/MI_Atlas_Green_E_02.MI_Atlas_Green_E_02")
      (else
        (Rendering|Material|SetMaterial _monitor1 1 "/Game/Low_Poly_Sci-Fi_Corridor/Materials/Alternate/White/MI_Atlas_White_E_01.MI_Atlas_White_E_01")))))

(fn ConstructionScript
  (bind _monitor1 (Variables|Default|GetMonitor1))
  (if (Variables|Default|GetIsLock)
    (Rendering|Material|SetMaterial _monitor1 1 "/Game/Low_Poly_Sci-Fi_Corridor/Materials/Alternate/Green/MI_Atlas_Green_E_02.MI_Atlas_Green_E_02")
    (else
      (Rendering|Material|SetMaterial _monitor1 1 "/Game/Low_Poly_Sci-Fi_Corridor/Materials/Alternate/White/MI_Atlas_White_E_01.MI_Atlas_White_E_01"))))