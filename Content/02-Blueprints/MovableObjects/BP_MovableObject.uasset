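; BP_MovableObject is a physics prop that reacts to impacts and exposes toggles for its mesh collision.
; On hit, optional behaviors trigger Chaos destruction, destroy the prop if fragile, and emit an AI alert sound.
; Velocity along the hit normal drives the fragility check and alert radius.
; Chaos targets are matched by GeometryCollectionActor name prefix, then an FS_MasterField is spawned and triggered before the hit actor is destroyed.
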(event OnComponentHit(Mesh)
  (params (HitComponent :type Primitive%20Component%20Object%20Reference) (OtherActor :type Actor%20Object%20Reference) (OtherComp :type Primitive%20Component%20Object%20Reference) (NormalImpulse :type Vector :default "0, 0, 0") (Hit :type Hit%20Result%20Structure%20%28by%20ref%29))
  (bind _returnvalue (Transformation|GetVelocity))
  (bind _returnvalue_2 (Math|Vector|Normalize (.normal Hit)))
  (bind _returnvalue_3 (Math|Vector|DotProduct _returnvalue_2 _returnvalue))
  (Utilities|FlowControl|Sequence
    (:then_0
      (if (Variables|Default|GetCan%20destroy%20Chaos)
        (|DestroyChaos OtherActor OtherActor (.location Hit))))
    (:then_1
      (if (Variables|Default|GetIs%20fragile)
        (if (< (* (Variables|Default|GetCollision%20Resistance) 10) _returnvalue_3)
          (Actor|DestroyActor))))
    (:then_2
      (if (Variables|Default|GetMake%20Collision%20Sound)
        (Default|AIAlertSound (Variables|Default|GetBPC_MakeAlertSound) (* _returnvalue_3 (/ (Variables|Default|GetCollision%20Sound%20Alert%20Radius) 1e+02)) (Variables|Default|GetCollision%20Sound%20Cue))))))

(fn ConstructionScript)

(fn EnablePhysicsCollision
  (Collision|SetCollisionEnabled (Variables|Default|GetMesh) "QueryAndPhysics"))

(fn DisablePhysicsCollision
  (Collision|SetCollisionEnabled (Variables|Default|GetMesh) "NoCollision"))