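; BP_Projectile is a projectile actor that kills BP_Guardian1 enemies and removes itself after a short lifespan.
; Its Sphere1 component destroys the projectile on any hit, and on overlap with a guardian destroys both actors.
; In the "test" level, that kill also spawns a replacement guardian at a fixed location and adds it to BP_Player's Enemis array.
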(event OnComponentBeginOverlap(Sphere1)
  (params (OverlappedComponent :type Primitive%20Component%20Object%20Reference) (OtherActor :type Actor%20Object%20Reference) (OtherComp :type Primitive%20Component%20Object%20Reference) (OtherBodyIndex :type Integer) (bFromSweep :type Boolean) (SweepResult :type Hit%20Result%20Structure%20%28by%20ref%29))
  (Utilities|FlowControl|Sequence
    (:then_0
      (bind _asbp_guardian_1 (Utilities|Casting|CastToBP_Guardian1 OtherActor))
      (Actor|DestroyActor _asbp_guardian_1)
      (Actor|DestroyActor)
      (bind _returnvalue (Game|GetCurrentLevelName true))
      (if (Utilities|Enum|Equal(Enum) _returnvalue "test")
        (bind _returnvalue_2 (Game|SpawnActorfromClass "/Game/IA/BP_Guardian1.BP_Guardian1_C" (Math|Transform|MakeTransform "330.000000,940.000000,130.000000" "0, 0, 0" "1.000000,1.000000,1.000000") "Undefined" "MultiplyWithRoot" 0 0))
        (bind _asbp_player (Utilities|Casting|CastToBP_Player (Game|Player|GetPlayerPawn 0)))
        (Utilities|Array|Add (Variables|/Game/02-Blueprints/BP_Player.BP_Player_C|GetEnemis _asbp_player) _returnvalue_2)))))

(event OnComponentHit(Sphere1)
  (params (HitComponent :type Primitive%20Component%20Object%20Reference) (OtherActor :type Actor%20Object%20Reference) (OtherComp :type Primitive%20Component%20Object%20Reference) (NormalImpulse :type Vector :default "0, 0, 0") (Hit :type Hit%20Result%20Structure%20%28by%20ref%29))
  (Actor|DestroyActor))

(event EventBeginPlay
  (Actor|SetLifeSpan 3.0))

(fn ConstructionScript)