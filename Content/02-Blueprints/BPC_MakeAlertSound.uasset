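; BPC_MakeAlertSound is a component that lets its owning actor make a noise that alerts nearby guardians.
; AIAlertSound plays the given sound at the owner's location and sphere-traces the given radius on the Pawn profile.
; Each BP_Guardian1 hit receives Alert with that location.
; A DoOnce throttles calls, resetting after a short Delay that runs only when a guardian is alerted.
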(event Custom|AI%20Alert%20Sound
  (params (Radius :type Float%20%28double-precision%29) (Sound%20Cue :type Sound%20Cue%20Object%20Reference))
  (bind _returnvalue (Components|GetOwner))
  (bind _returnvalue_2 (Transformation|GetActorLocation _returnvalue))
  (Utilities|FlowControl|DoOnce false :!label _label
    (:Completed
      (bind _outhits (Class|KismetSystemLibrary|SphereTraceMultibyProfile _returnvalue_2 _returnvalue_2 Radius "Pawn" false 0 "ForOneFrame" true "(R=1.000000,G=0.000000,B=0.000000,A=1.000000)" "(R=0.000000,G=1.000000,B=0.000000,A=1.000000)" 0.2))
      (Audio|PlaySoundatLocation Sound%20Cue _returnvalue_2 "0, 0, 0" 1.0 1.0 0.0 0 0 0 0)
      (for _array_element _outhits
        (bind _asbp_guardian_1 (Utilities|Casting|CastToBP_Guardian1 (.HitActor (Collision|BreakHitResult _array_element))))
        (Default|Alert _asbp_guardian_1 (Transformation|GetActorLocation (Components|GetOwner))))
      (Utilities|FlowControl|Delay 0.2)
      (goto _label Reset))))

(event EventBeginPlay)

(event EventTick
  (params (DeltaSeconds :type Float%20%28single-precision%29)))