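; Freeze projectile actor that damages Guardian enemies and leaves an ice crystal effect on them.
; It expires after a short lifespan or destroys itself when its sphere registers a hit.
; On sphere overlap with a BP_Guardian1, it applies a small amount of damage and spawns a Niagara ice crystal below the Guardian's center.
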(event OnComponentBeginOverlap(Sphere1)
  (params (OverlappedComponent :type Primitive%20Component%20Object%20Reference) (OtherActor :type Actor%20Object%20Reference) (OtherComp :type Primitive%20Component%20Object%20Reference) (OtherBodyIndex :type Integer) (bFromSweep :type Boolean) (SweepResult :type Hit%20Result%20Structure%20%28by%20ref%29))
  (Utilities|FlowControl|Sequence
    (:then_0
      (bind _asbp_guardian_1 (Utilities|Casting|CastToBP_Guardian1 OtherActor))
      (Game|Damage|ApplyDamage _asbp_guardian_1 2.0 0 0 "/Script/Engine.DamageType")
      (Niagara|SpawnSystematLocation (Variables|Default|GetNiagara%20Ice%20Crystal) (- (Transformation|GetActorLocation _asbp_guardian_1) "0.000000,0.000000,80.000000")))))

(event OnComponentHit(Sphere1)
  (params (HitComponent :type Primitive%20Component%20Object%20Reference) (OtherActor :type Actor%20Object%20Reference) (OtherComp :type Primitive%20Component%20Object%20Reference) (NormalImpulse :type Vector :default "0, 0, 0") (Hit :type Hit%20Result%20Structure%20%28by%20ref%29))
  (Actor|DestroyActor))

(event EventBeginPlay
  (Actor|SetLifeSpan 3.0))

(fn ConstructionScript)