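; BP_Camera1 is a sweeping security camera that raises an alert when the player enters its detection cone.
; A CameraSweep component swings it between left and right limits, pausing two seconds at each before restarting.
; Cone overlap with BP_Player dispatches an alert carrying the player's location and plays an alert sound.
; Each sweep layers start, middle and end turning sounds, timed from the sweep duration.
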(event OnComponentBeginOverlap(Cone)
  (params (OverlappedComponent :type Primitive%20Component%20Object%20Reference) (OtherActor :type Actor%20Object%20Reference) (OtherComp :type Primitive%20Component%20Object%20Reference) (OtherBodyIndex :type Integer) (bFromSweep :type Boolean) (SweepResult :type Hit%20Result%20Structure%20%28by%20ref%29))
  ;[0.15 0.15 0.15 0.5] Détection du joueur
  (Utilities|Casting|CastToBP_Player OtherActor)
  (Default|CallAlertDispatch (Transformation|GetActorLocation (Game|GetPlayerCharacter 0)))
  (Audio|Components|Audio|Play (Variables|Default|GetAlertSound) 0.0))

(event OnReachedLeftLimit(CameraSweep)
  (Class|CameraSweepComponent|StopSweep (Variables|Default|GetCameraSweep))
  (Utilities|FlowControl|Delay 2.0)
  (CallFunction|PlayTurnCameraSound)
  (Class|CameraSweepComponent|StartSweep (Variables|Default|GetCameraSweep)))

(event OnReachedRightLimit(CameraSweep)
  (Class|CameraSweepComponent|StopSweep (Variables|Default|GetCameraSweep))
  (Utilities|FlowControl|Delay 2.0)
  (CallFunction|PlayTurnCameraSound)
  (Class|CameraSweepComponent|StartSweep (Variables|Default|GetCameraSweep)))

(event Custom|PlayTurnCameraSound
  (bind _middleturncamerasound (Variables|Default|GetMiddleTurnCameraSound))
  (Audio|Components|Audio|Play (Variables|Default|GetStartTurnCameraSound) 0.0)
  (Audio|Components|Audio|Play _middleturncamerasound 0.0)
  (Utilities|FlowControl|Delay (- (Variables|/Script/FileRouge.CameraSweepComponent|GetDuration (Variables|Default|GetCameraSweep)) 1.0))
  (Audio|Components|Audio|Stop _middleturncamerasound)
  (Audio|Components|Audio|Play (Variables|Default|GetEndTurnCameraSound) 0.0))

(event EventBeginPlay
  ;[0.15 0.15 0.15 0.5] BeginPlay
  (CallFunction|PlayTurnCameraSound)
  (Class|CameraSweepComponent|StartSweep (Variables|Default|GetCameraSweep)))

(fn ConstructionScript)