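; Security camera that sweeps between yaw limits via a CameraSweep component, pausing at each limit with timed motor sounds, unless Shutdown at BeginPlay.
; A looping timer checks the Cone for the player and confirms line of sight by sphere trace.
; Detection dispatches the player's location, sounds the alarm and pauses detection, not the sweep, for AlarmDuration.
; Debug leftovers remain: per-tick yaw print and trace drawing.
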(event OnComponentBeginOverlap(Cone)
  (params (OverlappedComponent :type Primitive%20Component%20Object%20Reference) (OtherActor :type Actor%20Object%20Reference) (OtherComp :type Primitive%20Component%20Object%20Reference) (OtherBodyIndex :type Integer) (bFromSweep :type Boolean) (SweepResult :type Hit%20Result%20Structure%20%28by%20ref%29)))

(event OnReachedLeftLimit(CameraSweep)
  ;[0.15 0.15 0.15 0.5] Turn Camera
  (Class|CameraSweepComponent|StopSweep (Variables|Default|GetCameraSweep))
  (Utilities|FlowControl|Delay 2.0)
  (CallFunction|PlayTurnCameraSound)
  (Class|CameraSweepComponent|StartSweep (Variables|Default|GetCameraSweep)))

(event OnReachedRightLimit(CameraSweep)
  ;[0.15 0.15 0.15 0.5] Turn Camera
  (Class|CameraSweepComponent|StopSweep (Variables|Default|GetCameraSweep))
  (Utilities|FlowControl|Delay 2.0)
  (CallFunction|PlayTurnCameraSound)
  (Class|CameraSweepComponent|StartSweep (Variables|Default|GetCameraSweep)))

(event Custom|CustomEvent
  (bind _returnvalue (Game|Player|GetPlayerPawn 0))
  (bind _returnvalue_2 (Transformation|GetActorLocation _returnvalue))
  ;[0.15 0.15 0.15 0.5] Détection du joueur
  (for _array_element (Collision|GetOverlappingActors (Variables|Default|GetCone) "/Game/02-Blueprints/Player/BP_Player.BP_Player_C" :!class /Script/Engine.PrimitiveComponent)
    (if (== _array_element _returnvalue)
      (bind _outhit (Collision|SphereTraceByChannel (Transformation|GetWorldLocation (Variables|Default|GetCube)) _returnvalue_2 1e+01 "TraceTypeQuery1" false 0 "ForDuration"))
      (if (== (.HitActor (Collision|BreakHitResult _outhit)) (Game|Player|GetPlayerPawn 0))
        (Default|CallAlertDispatch _returnvalue_2)
        (Audio|Components|Audio|Play (Variables|Default|GetAlertSound) 0.0)
        (Utilities|Time|PauseTimerbyHandle (Variables|Default|GetCamera%20Update%20Handler))
        (Variables|Default|SetAlarm%20On true)
        (Utilities|FlowControl|Delay (Variables|Default|GetAlarm%20Duration))
        (Variables|Default|SetAlarm%20On false)
        (Utilities|Time|UnpauseTimerbyHandle (Variables|Default|GetCamera%20Update%20Handler))
        (Audio|Components|Audio|Stop (Variables|Default|GetAlertSound))))))

(event Custom|PlayTurnCameraSound
  (bind _middleturncamerasound (Variables|Default|GetMiddleTurnCameraSound))
  ;[0.15 0.15 0.15 0.5] Play Sound Camera
  (Audio|Components|Audio|Play (Variables|Default|GetStartTurnCameraSound) 0.0)
  (Audio|Components|Audio|Play _middleturncamerasound 0.0)
  (Utilities|FlowControl|Delay (- (Variables|/Script/FileRouge.CameraSweepComponent|GetDuration (Variables|Default|GetCameraSweep)) 1.0))
  (Audio|Components|Audio|Stop _middleturncamerasound)
  (Audio|Components|Audio|Play (Variables|Default|GetEndTurnCameraSound) 0.0))

(event EventBeginPlay
  ;[0.15 0.15 0.15 0.5] BeginPlay
  (if (not (Variables|Default|GetShutdown?))
    (CallFunction|PlayTurnCameraSound)
    (Class|CameraSweepComponent|StartSweep (Variables|Default|GetCameraSweep))
    (bind _returnvalue (Utilities|Time|SetTimerbyEvent (delegate Custom|CustomEvent) 0.33 true true))
    (Variables|Default|SetCamera%20Update%20Handler _returnvalue)))

(event EventTick
  (params (DeltaSeconds :type Float%20%28single-precision%29))
  (bind _self self)
  (bind _camerasweep (Variables|Default|GetCameraSweep))
  (bind _returnvalue (Utilities|GetDisplayName _self))
  (Development|PrintString (Utilities|String|Append _returnvalue ":  
Current =" (Utilities|String|ToString(Float) (Variables|/Script/FileRouge.CameraSweepComponent|GetCurrentYaw _camerasweep)) " 
Target =" (Utilities|String|ToString(Float) (Variables|/Script/FileRouge.CameraSweepComponent|GetTargetYaw _camerasweep))) true true "(R=0.000000,G=0.660000,B=1.000000,A=1.000000)" 2.0 (Utilities|String|StringToName _returnvalue)))

(fn ConstructionScript)