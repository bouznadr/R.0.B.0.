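; BP_Labyrinth is a tilt-board ball maze minigame that completes Quest6 when won.
; Input axes rotate the board mesh each tick, R resets it, and Q returns possession to BP_Player.
; An overlap with BP_Ball triggers the win and unlock call.
; Losing plays an alarm and shows a lose widget, then EndAnimation exits and respawns the ball, briefly disabling collision damage on its Geometry Collection sphere.
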(event OnComponentBeginOverlap(CheckWin)
  (params (OverlappedComponent :type Primitive%20Component%20Object%20Reference) (OtherActor :type Actor%20Object%20Reference) (OtherComp :type Primitive%20Component%20Object%20Reference) (OtherBodyIndex :type Integer) (bFromSweep :type Boolean) (SweepResult :type Hit%20Result%20Structure%20%28by%20ref%29))
  ;[0.15 0.15 0.15 0.5] Voir si le joueur a gagné
  (bind _asbp_ball (Utilities|Casting|CastToBP_Ball OtherActor))
  (CallFunction|Win)
  (Class|GeometryCollectionComponent|SetEnableDamagefromCollision (Variables|/Game/02-Blueprints/Labyrinth/BP_Ball.BP_Ball_C|GetGC_Sphere _asbp_ball) false))

(event Custom|RotationReset
  ;[0.15 0.15 0.15 0.5] Reset de la rotation
  (if (not (Variables|Default|GetIsWin))
    (Transformation|SetRelativeRotation (Variables|Default|GetStaticMesh) "0, 0, 0" false false)))

(event Custom|Quit
  ;[0.15 0.15 0.15 0.5] Fonction Quitter
  (if (Variables|Default|GetIsGame)
    (Pawn|Possess (Game|GetPlayerController 0) (Variables|Default|GetPlayer))
    (CallFunction|RotationReset)
    (Widget|SetVisibility (Variables|/Game/02-Blueprints/Player/BP_Player.BP_Player_C|GetPlayer%20HUD (Variables|Default|GetPlayer)) "Visible")))

(event Custom|Lose
  ;[0.15 0.15 0.15 0.5] Fonction Lose
  (CallFunction|StopSound)
  (Utilities|FlowControl|Delay 0.2)
  (bind _returnvalue (Audio|SpawnSound2D "/Game/04-Assets/Audio/SFX/AlarmeAlerteCamera.AlarmeAlerteCamera" 0.1 1.0 0.0 0))
  (Variables|Default|SetSound _returnvalue)
  (bind _returnvalue_2 (UserInterface|CreateWidget "/Game/02-Blueprints/UI/WBP_LoseLabyrinth.WBP_LoseLabyrinth_C"))
  (bind _output_get (Variables|Default|SetLoseScreen _returnvalue_2))
  (Utilities|FlowControl|Delay 1.0)
  (UserInterface|Viewport|AddtoViewport _output_get 0))

(event Custom|Win
  ;[0.15 0.15 0.15 0.5] FonctionWin
  (CallFunction|StopSound)
  (Variables|Default|SetIsWin true)
  (CallFunction|Quit)
  (Variables|Default|SetIsGame false)
  (Default|CallUnlockAll)
  (Default|CompletedQuest (Variables|Default|GetPlayer) "Quest6"))

(event Custom|EndAnimation
  ;[0.15 0.15 0.15 0.5] A la fin de l'animation de défaite
  (Components|Activation|SetActive (Variables|Default|GetSound) false false)
  (bind _foundwidgets (Widget|GetAllWidgetsOfClass "/Game/02-Blueprints/UI/WBP_LoseLabyrinth.WBP_LoseLabyrinth_C" true))
  (for _array_element _foundwidgets
    (Widget|RemovefromParent _array_element)
    (CallFunction|Quit)
    (CallFunction|RespawnBall)
    (Variables|Default|SetIsGame false)))

(event Custom|Stop%20Sound
  ;[0.15 0.15 0.15 0.5] Stopper les battements de coeur
  (Components|Activation|SetActive (Variables|/Game/02-Blueprints/Labyrinth/BP_TriggerLabyrinth.BP_TriggerLabyrinth_C|GetHeartSound (Variables|Default|GetBP_TriggerLabyrinth)) false false))

(event Custom|RespawnBall
  ;[0.15 0.15 0.15 0.5] Respawn de la balle
  (Utilities|FlowControl|Delay 1.0)
  (bind _returnvalue (Game|SpawnActorfromClass "/Game/02-Blueprints/Labyrinth/BP_Ball.BP_Ball_C" (Math|Transform|MakeTransform (Transformation|GetActorLocation (Variables|Default|GetSpawnTargetPoint)) "0, 0, 0" "1.000000,1.000000,1.000000") "AlwaysSpawn" "MultiplyWithRoot" 0 0))
  (Class|GeometryCollectionComponent|SetEnableDamagefromCollision (Variables|/Game/02-Blueprints/Labyrinth/BP_Ball.BP_Ball_C|GetGC_Sphere _returnvalue) false)
  (Utilities|FlowControl|Delay 1.0)
  (Class|GeometryCollectionComponent|SetEnableDamagefromCollision (Variables|/Game/02-Blueprints/Labyrinth/BP_Ball.BP_Ball_C|GetGC_Sphere _returnvalue) true))

(event EventBeginPlay
  ;[0.15 0.15 0.15 0.5] Begin Play
  (bind _returnvalue (Actor|GetActorOfClass "/Game/02-Blueprints/Player/BP_Player.BP_Player_C"))
  (Variables|Default|SetPlayer _returnvalue)
  (bind _returnvalue_2 (Actor|GetActorOfClass "/Game/02-Blueprints/Labyrinth/BP_TriggerLabyrinth.BP_TriggerLabyrinth_C"))
  (Variables|Default|SetBP_TriggerLabyrinth _returnvalue_2))

(event EventTick
  (params (DeltaSeconds :type Float%20%28single-precision%29))
  ;[0.15 0.15 0.15 0.5] Rotation du plateau
  (Variables|Default|SetMouseY_Value (Input|EnhancedActionValues|GetIA_RotateY))
  (Variables|Default|SetMouseX_Value (Input|EnhancedActionValues|GetIA_RotateX))
  (Transformation|AddLocalRotation (Variables|Default|GetStaticMesh) (Math|Rotator|MakeRotator (.roll (Math|Rotator|MakeRotator (* (Variables|Default|GetMouseY_Value) (Variables|Default|GetRotationSpeed) DeltaSeconds -1.0) (* (Variables|Default|GetMouseX_Value) (Variables|Default|GetRotationSpeed) DeltaSeconds) 0.0)) (.pitch (Math|Rotator|MakeRotator (* (Variables|Default|GetMouseY_Value) (Variables|Default|GetRotationSpeed) DeltaSeconds -1.0) (* (Variables|Default|GetMouseX_Value) (Variables|Default|GetRotationSpeed) DeltaSeconds) 0.0)) 0.0) false false))

(event Input|KeyboardEvents|R
  (params (Key :type Key%20Structure :default "None"))
  ;[0.15 0.15 0.15 0.5] Bouton pour reset
  (:Pressed
    (CallFunction|RotationReset)))

(event Input|KeyboardEvents|Q
  (params (Key :type Key%20Structure :default "None"))
  ;[0.15 0.15 0.15 0.5] Quitter manuellement
  (:Pressed
    (CallFunction|Quit)))

(fn ConstructionScript)