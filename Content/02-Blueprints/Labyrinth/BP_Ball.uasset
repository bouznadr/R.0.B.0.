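; BP_Ball is the breakable ball of the labyrinth, whose destruction reports a win or a loss.
; When its GC_Sphere Geometry Collection fires a Chaos break event, it looks up BP_Labyrinth and reads its game state.
; During a game it calls Win or Lose based on IsWin; outside a game it only prints an access card message.
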(event OnChaosBreakEvent(GC_Sphere)
  (params (BreakEvent :type Chaos%20Break%20Event%20Structure%20%28by%20ref%29))
  ;[0.15 0.15 0.15 0.5] Quand la balle est cassé, voir si c'est un defaite ou une victoire ou bien la carte d'accès
  (bind _returnvalue (Actor|GetActorOfClass "/Game/02-Blueprints/Labyrinth/BP_Labyrinth.BP_Labyrinth_C"))
  (bind _output_get (Variables|Default|SetBP_Labyrinth _returnvalue))
  (if (Variables|/Game/02-Blueprints/Labyrinth/BP_Labyrinth.BP_Labyrinth_C|GetIsGame _output_get)
    (if (Variables|/Game/02-Blueprints/Labyrinth/BP_Labyrinth.BP_Labyrinth_C|GetIsWin (Variables|Default|GetBP_Labyrinth))
      (Default|Win (Variables|Default|GetBP_Labyrinth))
      (Variables|/Game/02-Blueprints/Labyrinth/BP_Labyrinth.BP_Labyrinth_C|SetIsWin (Variables|Default|GetBP_Labyrinth) true)
      (else
        (Default|Lose (Variables|Default|GetBP_Labyrinth))))
    (else
      (Development|PrintString "Carte d'acces"))))

(fn ConstructionScript)