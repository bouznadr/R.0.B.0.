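; Trigger box that switches the player into the labyrinth mini-game when BP_Player overlaps it.
; On BeginPlay it finds BP_Labyrinth in the level.
; On overlap, if the labyrinth is not yet won, it hides the player HUD, has the player controller possess the labyrinth, flags the game active and enables its tick.
; It then starts a 2D heartbeat sound and keeps a reference to it.
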(event OnComponentBeginOverlap(Box)
  (params (OverlappedComponent :type Primitive%20Component%20Object%20Reference) (OtherActor :type Actor%20Object%20Reference) (OtherComp :type Primitive%20Component%20Object%20Reference) (OtherBodyIndex :type Integer) (bFromSweep :type Boolean) (SweepResult :type Hit%20Result%20Structure%20%28by%20ref%29))
  ;[0.15 0.15 0.15 0.5] Récupération du player au contact avec la box
  (bind _asbp_player (Utilities|Casting|CastToBP_Player OtherActor))
  (Variables|Default|SetAs%20BP%20Player _asbp_player)
  (CallFunction|PossesLabyrinth))

(event Custom|PossesLabyrinth
  ;[0.15 0.15 0.15 0.5] Controler la plaque
  (if (not (Variables|/Game/02-Blueprints/Labyrinth/BP_Labyrinth.BP_Labyrinth_C|GetIsWin (Variables|Default|GetAS%20BP%20Labyrinth)))
    (Widget|SetVisibility (Variables|/Game/02-Blueprints/Player/BP_Player.BP_Player_C|GetPlayer%20HUD (Variables|Default|GetAs%20BP%20Player)) "Hidden")
    (Pawn|Possess (Game|GetPlayerController 0) (Variables|Default|GetAS%20BP%20Labyrinth))
    (Variables|/Game/02-Blueprints/Labyrinth/BP_Labyrinth.BP_Labyrinth_C|SetIsGame (Variables|Default|GetAS%20BP%20Labyrinth) true)
    (Actor|Tick|SetActorTickEnabled (Variables|Default|GetAS%20BP%20Labyrinth) true)
    (bind _returnvalue (Audio|SpawnSound2D "/Game/04-Assets/Audio/SFX/Heart.Heart" 1.0 1.0 0.0 0 false false))
    (Variables|Default|SetHeartSound _returnvalue)))

(event EventBeginPlay
  ;[0.15 0.15 0.15 0.5] Récupération de BP_Labyrinth
  (bind _returnvalue (Actor|GetActorOfClass "/Game/02-Blueprints/Labyrinth/BP_Labyrinth.BP_Labyrinth_C"))
  (Variables|Default|SetAS%20BP%20Labyrinth _returnvalue))

(fn ConstructionScript)