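; Collectible pickup Blueprint that grants the player freeze ammo.
; It overrides the UsePickedItem event to increment FreezeAmmo on the BPPlayer reference by one.
; It has no other active logic of its own: BeginPlay, overlap and Tick are disabled stubs, and the construction script only calls its parent.
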(event EventBeginPlay
  (|CallParentFunction) ; Ce nœud est désactivé et ne sera pas appelé.\nFaites glisser les broches pour générer des fonctionnalités.
)

(event Collision|EventActorBeginOverlap
  (params (OtherActor :type Actor%20Object%20Reference))
  (|CallParentFunction OtherActor) ; Ce nœud est désactivé et ne sera pas appelé.\nFaites glisser les broches pour générer des fonctionnalités.
)

(event EventTick
  (params (DeltaSeconds :type Float%20%28single-precision%29))
  (|CallParentFunction DeltaSeconds) ; Ce nœud est désactivé et ne sera pas appelé.\nFaites glisser les broches pour générer des fonctionnalités.
)

(event EventUsePickedItem
  (bind _bp_player (Variables|Default|GetBP%20Player))
  (Variables|/Game/02-Blueprints/Player/BP_Player.BP_Player_C|SetFreezeAmmo _bp_player (+ (Variables|/Game/02-Blueprints/Player/BP_Player.BP_Player_C|GetFreezeAmmo _bp_player) 1)))

(fn ConstructionScript
  (|CallParentFunction))