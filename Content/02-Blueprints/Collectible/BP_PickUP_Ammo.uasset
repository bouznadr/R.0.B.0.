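; BP_PickUP_Ammo is an ammo pickup that adds one regular ammo to the player when used.
; UsePickedItem also calls CompletedQuest for Quest4 and clears the player's objective object.
; Overlap events on its Sphere show the Icon when BP_Player enters and hide it when the player leaves.
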(event OnComponentEndOverlap(Sphere)
  (params (OverlappedComponent :type Primitive%20Component%20Object%20Reference) (OtherActor :type Actor%20Object%20Reference) (OtherComp :type Primitive%20Component%20Object%20Reference) (OtherBodyIndex :type Integer))
  (Utilities|Casting|CastToBP_Player OtherActor)
  (Rendering|SetVisibility (Variables|Default|GetIcon) false false))

(event OnComponentBeginOverlap(Sphere)
  (params (OverlappedComponent :type Primitive%20Component%20Object%20Reference) (OtherActor :type Actor%20Object%20Reference) (OtherComp :type Primitive%20Component%20Object%20Reference) (OtherBodyIndex :type Integer) (bFromSweep :type Boolean) (SweepResult :type Hit%20Result%20Structure%20%28by%20ref%29))
  (Utilities|Casting|CastToBP_Player OtherActor)
  (Rendering|SetVisibility (Variables|Default|GetIcon) true false))

(event EventBeginPlay
  (|CallParentFunction) ; Ce nœud est désactivé et ne sera pas appelé.\nFaites glisser les broches pour générer des fonctionnalités.
)

(event Collision|EventActorBeginOverlap
  (params (OtherActor :type Actor%20Object%20Reference))
  (|CallParentFunction OtherActor) ; Ce nœud est désactivé et ne sera pas appelé.\nFaites glisser les broches pour générer des fonctionnalités.
)

(event EventTick
  (params (DeltaSeconds :type Float%20%28single-precision%29))
  (|CallParentFunction DeltaSeconds) ; Ce nœud est désactivé et ne sera pas appelé.\nFaites glisser les broches pour générer des fonctionnalités.
)

(event EventUsePickedItem
  (bind _bp_player (Variables|Default|GetBP%20Player))
  (Variables|/Game/02-Blueprints/Player/BP_Player.BP_Player_C|SetRegularAmmo _bp_player (+ (Variables|/Game/02-Blueprints/Player/BP_Player.BP_Player_C|GetRegularAmmo _bp_player) 1))
  (Default|CompletedQuest _bp_player "Quest4")
  (Variables|/Game/02-Blueprints/Player/BP_Player.BP_Player_C|SetObjective%20Object _bp_player 0))

(fn ConstructionScript
  (|CallParentFunction))