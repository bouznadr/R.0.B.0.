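; BP_EnergySource is a collectible that supplies fuel to the escape ship.
; It caches the BP_EscapeShip found in the level on BeginPlay.
; Its PickUpItemEvent sets the ship's HasFuel flag and destroys the pickup, or prints a message and stays if the ship is already fueled.
; Overlap and Tick only forward to the parent class.
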(event EventBeginPlay
  (|CallParentFunction)
  (bind _returnvalue (Actor|GetActorOfClass "/Game/02-Blueprints/BP_EscapeShip.BP_EscapeShip_C"))
  (Variables|Default|SetShipRef _returnvalue))

(event Collision|EventActorBeginOverlap
  (params (OtherActor :type Actor%20Object%20Reference))
  (|CallParentFunction OtherActor))

(event EventTick
  (params (DeltaSeconds :type Float%20%28single-precision%29))
  (|CallParentFunction DeltaSeconds))

(event EventPickUpItemEvent
  (bind _shipref (Variables|Default|GetShipRef))
  (if (Variables|/Game/02-Blueprints/BP_EscapeShip.BP_EscapeShip_C|GetHasFuel? _shipref)
    (Development|PrintString "You already have fuel")
    (else
      (Variables|/Game/02-Blueprints/BP_EscapeShip.BP_EscapeShip_C|SetHasFuel? _shipref true)
      (Actor|DestroyActor))))

(fn ConstructionScript)