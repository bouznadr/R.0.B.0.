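; BP_DoorPadPressure is a sliding double corridor door that opens according to a weight percentage, apparently supplied by a pressure pad.
; CurrentWeightValues stores the target, either proportional or all-or-nothing when UpdateWhenComplete is set, flags IsComplete at full weight and enables Tick.
; Tick interpolates DoorOpenAmount toward the target, sliding both panels in opposite directions along local X.
; Tick disables itself once the open amount matches the target.
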(event EventCurrentWeightValues
  (params (Weight%20percent :type Float%20%28double-precision%29))
  (bind _returnvalue (== Weight%20percent 1.0))
  (if (Variables|Default|GetUpdate%20when%20complete%20)
    (Variables|Default|SetWeight%20Percent (Math|Conversions|ToFloat(Boolean) _returnvalue))
    (else
      (Variables|Default|SetWeight%20Percent Weight%20percent)))
  (Variables|Default|SetIsComplete _returnvalue)
  (Actor|Tick|SetActorTickEnabled true))

(event EventTick
  (params (DeltaSeconds :type Float%20%28single-precision%29))
  (if (== (Variables|Default|GetDoorOpenAmount) (Variables|Default|GetWeight%20Percent))
    (Actor|Tick|SetActorTickEnabled false)
    (else
      (Variables|Default|SetDoorOpenAmount (Math|Interpolation|FInterpTo (Variables|Default|GetDoorOpenAmount) (Variables|Default|GetWeight%20Percent) (Utilities|Time|GetWorldDeltaSeconds) 5.0))
      (Utilities|FlowControl|Sequence
        (:then_0
          ;[0.15 0.15 0.15 0.5] LeftDoor
          (Variables|Default|SetDoorleftLocation (Math|Vector|MakeVector (Math|Float|Lerp 0.0 8e+01 (Variables|Default|GetDoorOpenAmount)) 0.0 0.0))
          (Transformation|SetRelativeLocation (Variables|Default|GetSM_CoridorDoorLeft) (Variables|Default|GetDoorleftLocation) false false))
        (:then_1
          ;[0.15 0.15 0.15 0.5] Right door
          (Variables|Default|SetDoorrightLocation (Math|Vector|MakeVector (Math|Float|Lerp 0.0 -79.0 (Variables|Default|GetDoorOpenAmount)) 0.0 0.0))
          (Transformation|SetRelativeLocation (Variables|Default|GetSM_CoridorDoorRight) (Variables|Default|GetDoorrightLocation) false false))))))

(fn ConstructionScript)