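; Movable cube object that breaks Chaos geometry collections it collides with.
; On a Cube hit, it identifies geometry collection actors by an object-name prefix, then spawns an FS_MasterField at the impact point and fires it through CETrigger.
; After a short delay it destroys the stored geometry collection actor, while the spawned field is not cleaned up here.
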(event OnComponentHit(Cube)
  (params (HitComponent :type Primitive%20Component%20Object%20Reference) (OtherActor :type Actor%20Object%20Reference) (OtherComp :type Primitive%20Component%20Object%20Reference) (NormalImpulse :type Vector :default "0, 0, 0") (Hit :type Hit%20Result%20Structure%20%28by%20ref%29))
  (if (Utilities|Enum|Equal(Enum) (Utilities|String|GetSubstring (Utilities|GetObjectName OtherActor) 0 23) "GeometryCollectionActor")
    (Variables|Default|SetObject%20Destroy OtherActor)
    (bind _returnvalue (Game|SpawnActorfromClass "/Engine/EditorResources/FieldNodes/FS_MasterField.FS_MasterField_C" (Math|Transform|MakeTransform (.location Hit) "0, 0, 0" "1.000000,1.000000,1.000000") "Undefined" "MultiplyWithRoot" 0 0))
    (Variables|/Engine/EditorResources/FieldNodes/FS_MasterField.FS_MasterField_C|SetActivationType _returnvalue "NewEnumerator4")
    (Default|CETrigger _returnvalue)
    (Utilities|FlowControl|Delay 3.0)
    (Actor|DestroyActor (Variables|Default|GetObject%20Destroy))))

(event EventBeginPlay)

(event Collision|EventActorBeginOverlap
  (params (OtherActor :type Actor%20Object%20Reference)))

(event EventTick
  (params (DeltaSeconds :type Float%20%28single-precision%29)))

(fn ConstructionScript)